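; BP_Runner is a player-controlled character that runs constantly along world +X, with speed driven by tapping.
; BeginPlay adds the IMC_Runner Enhanced Input mapping context.
; Tick applies forward movement and steadily drains MaxWalkSpeed by SlowMultiplier per second, clamped at zero.
; Each PowerLeft or PowerRight press calls IncreaseSpeed, adding a fixed boost with no upper cap or enforced left-right alternation.
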(event `self.ReceiveBeginPlay`
  (bind _asplayer_controller (cast `PlayerController` (`self.GetController`)))
  (`EnhancedInputSubsystemInterface.AddMappingContext` (pcsubsystem `EnhancedInputLocalPlayerSubsystem` _asplayer_controller) "/Game/Input/IMC_Runner.IMC_Runner" 0 (struct)))

(event `self.ReceiveTick`
  (params (DeltaSeconds :type "Float (single-precision)"))
  (`self.AddMovementInput` (1.0 0.0 0.0))
  (set `CharacterMovementComponent.MaxWalkSpeed` (`KismetMathLibrary.FMax` (- (`CharacterMovementComponent.MaxWalkSpeed` (`self.CharacterMovement`)) (* DeltaSeconds (`self.SlowMultiplier`)))) (`self.CharacterMovement`)))

(event `EnhancedInput|/Game/Input/Actions/IA_PowerLeft`
  (params (ActionValue :type Boolean) (ElapsedSeconds :type "Float (double-precision)") (TriggeredSeconds :type "Float (double-precision)") (InputAction :type "InputAction Object Reference" :default "/Game/Input/Actions/IA_PowerLeft.IA_PowerLeft"))
  (:`Started`
    (`self.IncreaseSpeed`)))

(event `EnhancedInput|/Game/Input/Actions/IA_PowerRight`
  (params (ActionValue :type Boolean) (ElapsedSeconds :type "Float (double-precision)") (TriggeredSeconds :type "Float (double-precision)") (InputAction :type "InputAction Object Reference" :default "/Game/Input/Actions/IA_PowerRight.IA_PowerRight"))
  (:`Started`
    (`self.IncreaseSpeed`)))

(fn `IncreaseSpeed`
  (set `CharacterMovementComponent.MaxWalkSpeed` (+ (`CharacterMovementComponent.MaxWalkSpeed` (`self.CharacterMovement`)) (`self.SpeedIncreasePerTap`)) (`self.CharacterMovement`)))

(fn `UserConstructionScript`)